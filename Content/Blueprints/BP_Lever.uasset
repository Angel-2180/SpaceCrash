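; VR-style lever actor that follows a grabbable handle and plays a sound when pulled to its activated position.
; Each Tick passes the pivot, inner and outer spheres and grabbable to UpdateLeverRotation, then tests the pivot with IsLeverActivated.
; The first activation latches LeverDown, which is never reset here, so the sound plays once.
; An unconnected look-at rotation with clamped pitch remains in the graph.
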(event `self.ReceiveBeginPlay`
  (set `LeverGrabbable.PreviousParent` (`self.Scene1`) (`self.BP_LeverGrabbable`)))

(event `self.ReceiveTick`
  (params (DeltaSeconds :type "Float (single-precision)"))
  (bind _scene (`self.Scene`))
  (`self.UpdateLeverRotation` _scene (`self.OutterSphere`) (`self.InnerSphere`) (`self.BP_LeverGrabbable`))
  (bind _returnvalue (`self.IsLeverActivated` _scene))
  (if (and _returnvalue (not (`self.LeverDown`)))
    (set `self.LeverDown` true)
    (`AudioComponent.Play` (`self.LeverDownSound`) 0.0)))

(fn `UserConstructionScript`)