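; BP_DoorEngine is a generator actor that presents its remaining energy and power state through a widget and sound.
; Every Tick it pushes TotalEnergyRemaining to its WBP_EngineSlider widget, skipping all other logic if that cast fails.
; Boolean flags act as one-shot triggers for backup and shutdown sounds, each also reporting an AI noise event at the sound's location.
; A near-power-down warning sound plays while energy is low and stops outside that range.
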(event `self.ReceiveBeginPlay`)

(event `self.ReceiveTick`
  (params (DeltaSeconds :type "Float (single-precision)"))
  (bind _generatornearpowerdown (`self.GeneratorNearPowerDown`))
  (bind _totalenergyremaining (`self.TotalEnergyRemaining`))
  (bind _generatordown (`self.GeneratorDown`))
  (bind _generatorbackup (`self.GeneratorBackup`))
  (bind _returnvalue (`AudioComponent.IsPlaying` _generatornearpowerdown))
  (bind _aswbp_engine_slider (cast `/Game/Blueprints/WBP_EngineSlider` (`WidgetComponent.GetWidget` (`self.Widget`))))
  (`/Game/Blueprints/WBP_EngineSlider.SetEnginePower` _aswbp_engine_slider _totalenergyremaining)
  (`|ExecutionSequence`
    (:`then_0`
      (if (`self.PlayEngineBackUpSound`)
        (set `self.PlayEngineBackUpSound` false)
        (`AudioComponent.Play` _generatorbackup 0.0)
        (`AISense_Hearing.ReportNoiseEvent` (`SceneComponent.K2_GetComponentLocation` _generatorbackup) 2.0 self 0.0 "Noise")))
    (:`then_1`
      (if (`self.PlayEngineShutDownSound`)
        (set `self.PlayEngineShutDownSound` false)
        (`AudioComponent.Play` _generatordown 0.0)
        (`AISense_Hearing.ReportNoiseEvent` (`SceneComponent.K2_GetComponentLocation` _generatordown) 2.0 self 0.0 "Noise")))
    (:`then_2`
      (if (and (<= _totalenergyremaining 25.0) (>= _totalenergyremaining 0.0))
        (if (not _returnvalue)
          (`AudioComponent.Play` _generatornearpowerdown 0.0))
        (elif _returnvalue
          (`AudioComponent.Stop` _generatornearpowerdown))))))

(fn `UserConstructionScript`)