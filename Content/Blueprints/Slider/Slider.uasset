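; Slider actor that tracks progress while actors overlap its button and signals completion with a sound.
; Button overlap events pass the actor to begin and end handlers, while Tick runs an update and broadcasts progress, both relying on logic defined outside this graph.
; SetProgress drives a material scalar on the slider mesh.
; Once activated, it plays the completion sound a single time and reports a tagged noise event at that location.
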(event `self.BUtton.OnComponentBeginOverlap`
  (params (OverlappedComponent :type "PrimitiveComponent Object Reference") (OtherActor :type "Actor Object Reference") (OtherComp :type "PrimitiveComponent Object Reference") (OtherBodyIndex :type Integer) (bFromSweep :type Boolean) (SweepResult :type "HitResult Structure (by ref)"))
  (`self.BeginOverLapping` OtherActor))

(event `self.BUtton.OnComponentEndOverlap`
  (params (OverlappedComponent :type "PrimitiveComponent Object Reference") (OtherActor :type "Actor Object Reference") (OtherComp :type "PrimitiveComponent Object Reference") (OtherBodyIndex :type Integer))
  (`self.EndOverLapping` OtherActor))

(event `self.ReceiveTick`
  (params (DeltaSeconds :type "Float (single-precision)"))
  (bind _completedsound (`self.CompletedSound`))
  (`self.Update`)
  (`self.ProgressChanged` (`self.Progress`))
  (if (and (`self.bActivated`) (not (`self.SoundPlayed`)))
    (set `self.SoundPlayed` true)
    (`AudioComponent.Play` _completedsound 0.0)
    (`AISense_Hearing.ReportNoiseEvent` (`SceneComponent.K2_GetComponentLocation` _completedsound) 1.0 self 0.0 "Noise")))

(fn `SetProgress`
  (params (Progress :type "Float (double-precision)"))
  (`MeshComponent.SetScalarParameterValueOnMaterials` (`self.Slider`) "Progress" Progress))

(fn `UserConstructionScript`)