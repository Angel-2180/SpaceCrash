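; BP_SpaceCraftDoor is a spacecraft door Blueprint that handles the sound, AI noise and indicator lights for opening and closing.
; Tick polls two one-shot flags, PlayDoorOpeningSound and PlayDoorClosingSound, clearing each as it fires; nothing here sets them or moves the door.
; Each plays its sound, reports a noise event at that location and swaps the lights: red on opening, green on closing.
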(event `self.ReceiveBeginPlay`)

(event `self.ReceiveTick`
  (params (DeltaSeconds :type "Float (single-precision)"))
  (bind _dooropeningsound (`self.DoorOpeningSound`))
  (bind _doorclosingsound (`self.DoorClosingSound`))
  (`|ExecutionSequence`
    (:`then_0`
      (if true
        (if (`self.PlayDoorOpeningSound`)
          (set `self.PlayDoorOpeningSound` false)
          (`AudioComponent.Play` _dooropeningsound 0.0)
          (`AISense_Hearing.ReportNoiseEvent` (`SceneComponent.K2_GetComponentLocation` _dooropeningsound) 2.0 self 0.0 "Noise")
          (`SceneComponent.SetVisibility` (`self.RedLight`) true false)
          (`SceneComponent.SetVisibility` (`self.GreenLight`) false false))))
    (:`then_1`
      (if (`self.PlayDoorClosingSound`)
        (set `self.PlayDoorClosingSound` false)
        (`AudioComponent.Play` _doorclosingsound 0.0)
        (`AISense_Hearing.ReportNoiseEvent` (`SceneComponent.K2_GetComponentLocation` _doorclosingsound) 2.0 self 0.0 "Noise")
        (`SceneComponent.SetVisibility` (`self.RedLight`) false false)
        (`SceneComponent.SetVisibility` (`self.GreenLight`) true false)))))

(fn `UserConstructionScript`)