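; Behavior tree decorator that starts the survival minigame on the alien AI.
; Its condition check casts the controlled pawn to BP_Alien, calls EnterSurvivalMinigame and returns true, so it acts as a side-effect trigger rather than a real test.
; A disconnected leftover chain would spawn hand trigger actors at the VR pawn's motion controllers, assign them to the alien and flag the minigame active.
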(fn `PerformConditionCheckAI`
  (params (OwnerController :type "AIController Object Reference") (ControlledPawn :type "Pawn Object Reference"))
  (returns (ReturnValue :type Boolean))
  (bind _asbp_alien (cast `/Game/Blueprints/BP_Alien` ControlledPawn))
  (`AlienController.EnterSurvivalMinigame` _asbp_alien)
  (return true))