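; BP_Alien is an AI alien in a VR game that detects the player by sight of the VR camera and by hearing.
; BeginPlay stores its detection, door-banging, random-noise, footstep and breath audio components in variables and silences them.
; Tick feeds the VR pawn's camera to UpdatePlayerDetection, while AI perception updates pass the blackboard to UpdateAIWithSound.
; Both detection functions are defined outside this file.
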(event `self.ReceiveBeginPlay`
  (set `self.AudioPlayerDetection` (`self.AudioDetectionSound`))
  (set `self.AudioPlayerDoorBanging` (`self.DoorBangingSound`))
  (set `self.AudioPlayerRandomNoise` (`self.AudioRandomSound`))
  (set `self.AudioPlayerFeet` (`self.AudioFeet`))
  (set `self.AudioPlayerBreath` (`self.AudioBreathSound`))
  (`AudioComponent.Stop` (`self.DoorBangingSound`))
  (`AudioComponent.Stop` (`self.AudioDetectionSound`))
  (`AudioComponent.Stop` (`self.AudioRandomSound`))
  (`AudioComponent.Stop` (`self.AudioFeet`))
  (`AudioComponent.Stop` (`self.AudioBreathSound`)))

(event `self.ReceiveTick`
  (params (DeltaSeconds :type "Float (single-precision)"))
  (bind _asbp_vrpawn (cast `/Game/Blueprints/BP_VRPawn` (`GameplayStatics.GetPlayerPawn` 0)))
  (`self.UpdatePlayerDetection` (`/Game/Blueprints/BP_VRPawn.Camera` _asbp_vrpawn)))

(event `self.AIPerception.OnTargetPerceptionUpdated`
  (params (Actor :type "Actor Object Reference") (Stimulus :type "AIStimulus Structure"))
  ;[1 1 1] HearingDetection
  (`self.UpdateAIWithSound` (`AIBlueprintHelperLibrary.GetBlackboard` null)))

(fn `UserConstructionScript`)