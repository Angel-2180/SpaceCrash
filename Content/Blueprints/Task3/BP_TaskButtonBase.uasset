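; Base task button actor that plays a completion sound and makes a noise for AI hearing.
; Tick polls the PlayActiveSound flag, which this graph never sets, and latches PlayCompletedSound so the response fires only once.
; It then plays CompletedSound and reports a "Noise"-tagged noise event at that component's location, with itself as instigator.
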(event `self.ReceiveTick`
  (params (DeltaSeconds :type "Float (single-precision)"))
  (bind _completedsound (`self.CompletedSound`))
  (if (and (`self.bPlayActiveSound`) (not (`self.PlayCompletedSound`)))
    (set `self.PlayCompletedSound` true)
    (`AudioComponent.Play` _completedsound 0.0)
    (`AISense_Hearing.ReportNoiseEvent` (`SceneComponent.K2_GetComponentLocation` _completedsound) 2.0 self 0.0 "Noise")))

(fn `UserConstructionScript`)