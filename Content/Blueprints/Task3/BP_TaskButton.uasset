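; BP_TaskButton is a task button actor that plays activation and deactivation sounds and makes them register as AI noise events.
; Tick polls the PlayActiveSound and PlayDeactiveSound flags, clearing each when set and playing its matching audio component.
; Each sound also reports a "Noise" event at that component's location, with the button as instigator.
; The flags are not set within this graph.
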(event `self.ReceiveTick`
  (params (DeltaSeconds :type "Float (single-precision)"))
  (bind _activesound (`self.ActiveSound`))
  (bind _nonactivesound (`self.NonActiveSound`))
  (`|ExecutionSequence`
    (:`then_0`
      (if (`self.bPlayActiveSound`)
        (set `self.bPlayActiveSound` false)
        (`AudioComponent.Play` _activesound 0.0)
        (`AISense_Hearing.ReportNoiseEvent` (`SceneComponent.K2_GetComponentLocation` _activesound) 2.0 self 0.0 "Noise")))
    (:`then_1`
      (if (`self.bPlayDeactiveSound`)
        (set `self.bPlayDeactiveSound` false)
        (`AudioComponent.Play` _nonactivesound 0.0)
        (`AISense_Hearing.ReportNoiseEvent` (`SceneComponent.K2_GetComponentLocation` _nonactivesound) 2.0 self 0.0 "Noise")))))

(fn `UserConstructionScript`)