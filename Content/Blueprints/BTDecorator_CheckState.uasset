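; Behavior tree decorator that gates its branch on the AI's current state.
; It passes when the blackboard enum in the State key equals the configurable StateToCheck value, comparing both as integers in PerformConditionCheckAI.
; The event graph holds only an unused leftover check of the State key against zero.
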(fn `PerformConditionCheckAI`
  (params (OwnerController :type "AIController Object Reference") (ControlledPawn :type "Pawn Object Reference"))
  (returns (ReturnValue :type Boolean))
  (return (== (`KismetMathLibrary.Conv_ByteToInt` (`BTFunctionLibrary.GetBlackboardValueAsEnum` (`self.State`))) (`KismetMathLibrary.Conv_ByteToInt` (`self.StateToCheck`)))))