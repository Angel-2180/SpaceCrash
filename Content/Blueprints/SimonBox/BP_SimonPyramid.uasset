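; Physical prop for a Simon box puzzle that plays fail and success sounds and makes noise when dropped or knocked.
; Tick polls one-shot flags, presumably set externally, to trigger the result sounds, and caches the mesh velocity.
; Hard hits play a random drop sound with volume scaled by the cached pre-impact speed.
; Each of these sounds also reports a noise event that AI can hear.
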(event `self.ReceiveBeginPlay`
  (`AudioComponent.Stop` (`self.Fail`))
  (`AudioComponent.Stop` (`self.Success`)))

(event `self.ReceiveTick`
  (params (DeltaSeconds :type "Float (single-precision)"))
  (bind _success (`self.Success`))
  (bind _fail (`self.Fail`))
  (set `self.LastFrameVelocity` (`SceneComponent.GetComponentVelocity` (`self.BaseMesh`)))
  (`|ExecutionSequence`
    (:`then_0`
      (if (`self.bPlayFailedSound`)
        (set `self.bPlayFailedSound` false)
        (`AudioComponent.Play` _fail 0.0)
        (`AISense_Hearing.ReportNoiseEvent` (`SceneComponent.K2_GetComponentLocation` _fail) 2.0 self 0.0 "Noise")))
    (:`then_1`
      (if (`self.bPlayCompletedSound`)
        (set `self.bPlayCompletedSound` false)
        (`AudioComponent.Play` _success 0.0)
        (`AISense_Hearing.ReportNoiseEvent` (`SceneComponent.K2_GetComponentLocation` _success) 2.0 self 0.0 "Noise")))))

(event `self.BaseMesh.OnComponentHit`
  (params (HitComponent :type "PrimitiveComponent Object Reference") (OtherActor :type "Actor Object Reference") (OtherComp :type "PrimitiveComponent Object Reference") (NormalImpulse :type "Vector Structure") (Hit :type "HitResult Structure (by ref)"))
  (bind _groundhit (`self.GroundHit`))
  (bind _returnvalue (`KismetMathLibrary.VSize` (`self.LastFrameVelocity`)))
  (if (> _returnvalue 200.0)
    (if (not (`AudioComponent.IsPlaying` _groundhit))
      (bind _returnvalue_2 (`DroppableSoundComponent.SetRandomDropSound` (`self.DroppableSound`)))
      (`AudioComponent.SetSound` _groundhit _returnvalue_2)
      (`AudioComponent.SetVolumeMultiplier` _groundhit (/ _returnvalue 1000.0))
      (`AudioComponent.Play` _groundhit 0.0)
      (`AISense_Hearing.ReportNoiseEvent` (`SceneComponent.K2_GetComponentLocation` _groundhit) 1.0 self 2000.0 "Noise"))))

(fn `UserConstructionScript`)