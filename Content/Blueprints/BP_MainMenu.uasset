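; Main menu actor with collision-driven Start, Quit, Credit and MainMenu buttons, triggered only by BP_IndexCollision overlaps.
; Credit and MainMenu swap the menu and credit panels, while Quit exits the game.
; Start hides the menu, launches a meteor-rain Niagara effect with sound, then plays a fade-to-black sequence before opening AlienTest.
; Once started, Tick steadily ramps the effect's velocity and explosion speed parameters to build acceleration.
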(event `self.ReceiveTick`
  (params (DeltaSeconds :type "Float (single-precision)"))
  (bind _returnvalue (* DeltaSeconds 3.0))
  (bind _ns_meteorrain (`self.NS_MeteorRain`))
  (if (`self.Play`)
    (bind _output_get (set `self.NewVelocity` (+ (`self.NewVelocity`) _returnvalue)))
    (`FXSystemComponent.SetVectorParameter` _ns_meteorrain "User.Velocity" (`KismetMathLibrary.MakeVector` _output_get))
    (bind _output_get_2 (set `self.NewExplosionSpeed` (+ (`self.NewExplosionSpeed`) _returnvalue)))
    (`FXSystemComponent.SetFloatParameter` _ns_meteorrain "User.ExplosionSpeed" _output_get_2)))

(event `self.Start.OnComponentBeginOverlap`
  (params (OverlappedComponent :type "PrimitiveComponent Object Reference") (OtherActor :type "Actor Object Reference") (OtherComp :type "PrimitiveComponent Object Reference") (OtherBodyIndex :type Integer) (bFromSweep :type Boolean) (SweepResult :type "HitResult Structure (by ref)"))
  (cast `/Game/Blueprints/BP_IndexCollision` OtherActor)
  (set `self.Play` true)
  (`SceneComponent.SetVisibility` (`self.MenuPanel`) false true)
  (`ActorComponent.Activate` (`self.NS_MeteorRain`) false)
  (`GameplayStatics.PlaySound2D` "/Game/AssetsToPush/Sounds/SpaceShip/spaceship-superspeed.spaceship-superspeed" 1.0 1.0 0.0 null null)
  (`KismetSystemLibrary.Delay` 15.0)
  (set `self.Fade` true)
  (bind (_outactor _returnvalue) (`LevelSequencePlayer.CreateLevelSequencePlayer` "/Game/AssetsToPush/FadeOutBlack.FadeOutBlack"))
  (`MovieSceneSequencePlayer.Play` _returnvalue)
  (`KismetSystemLibrary.Delay` 6.0)
  (`GameplayStatics.OpenLevel` "AlienTest"))

(event `self.Quit.OnComponentBeginOverlap`
  (params (OverlappedComponent :type "PrimitiveComponent Object Reference") (OtherActor :type "Actor Object Reference") (OtherComp :type "PrimitiveComponent Object Reference") (OtherBodyIndex :type Integer) (bFromSweep :type Boolean) (SweepResult :type "HitResult Structure (by ref)"))
  (cast `/Game/Blueprints/BP_IndexCollision` OtherActor)
  (`KismetSystemLibrary.QuitGame` null "Quit"))

(event `self.Credit.OnComponentBeginOverlap`
  (params (OverlappedComponent :type "PrimitiveComponent Object Reference") (OtherActor :type "Actor Object Reference") (OtherComp :type "PrimitiveComponent Object Reference") (OtherBodyIndex :type Integer) (bFromSweep :type Boolean) (SweepResult :type "HitResult Structure (by ref)"))
  (cast `/Game/Blueprints/BP_IndexCollision` OtherActor)
  (`SceneComponent.SetVisibility` (`self.CreditPanel`) true true)
  (`SceneComponent.SetVisibility` (`self.MenuPanel`) false true))

(event `self.MainMenu.OnComponentBeginOverlap`
  (params (OverlappedComponent :type "PrimitiveComponent Object Reference") (OtherActor :type "Actor Object Reference") (OtherComp :type "PrimitiveComponent Object Reference") (OtherBodyIndex :type Integer) (bFromSweep :type Boolean) (SweepResult :type "HitResult Structure (by ref)"))
  (cast `/Game/Blueprints/BP_IndexCollision` OtherActor)
  (`SceneComponent.SetVisibility` (`self.CreditPanel`) false true)
  (`SceneComponent.SetVisibility` (`self.MenuPanel`) true true))

(fn `UserConstructionScript`)