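; Behavior tree decorator that checks whether a spacecraft door is open for an alien AI.
; It reads the door from a blackboard key and returns that door's IsOpen flag, after confirming the pawn is an alien.
; An unused comparison of door mesh height against the alien's head height remains in the graph.
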(fn `PerformConditionCheckAI`
  (params (OwnerController :type "AIController Object Reference") (ControlledPawn :type "Pawn Object Reference"))
  (returns (ReturnValue :type Boolean))
  (bind _asbp_alien (cast `/Game/Blueprints/BP_Alien` ControlledPawn))
  (bind _asbp_space_craft_door (cast `/Game/Blueprints/BP_SpaceCraftDoor` (`BTFunctionLibrary.GetBlackboardValueAsObject` (`self.Door`))))
  (return (`SpaceCraftDoor.IsOpen` _asbp_space_craft_door)))