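; Passcode puzzle actor that plays its failed, completed and button sounds and makes each one audible to AI.
; Tick polls three boolean flags, clearing each one when set and playing the matching audio component.
; Each sound also reports an AI hearing noise event at its location, tagged "Noise", with a limited range.
; The passcode logic and whatever sets the flags are not in these graphs.
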(event `self.ReceiveBeginPlay`)

(event `self.ReceiveTick`
  (params (DeltaSeconds :type "Float (single-precision)"))
  (bind _failedsound (`self.FailedSound`))
  (bind _completedsound (`self.CompletedSound`))
  (bind _buttonsound (`self.ButtonSound`))
  (`|ExecutionSequence`
    (:`then_0`
      (if (`self.PlayFailedSound`)
        (set `self.PlayFailedSound` false)
        (`AudioComponent.Play` _failedsound 0.0)
        (`AISense_Hearing.ReportNoiseEvent` (`SceneComponent.K2_GetComponentLocation` _failedsound) 1.0 self 1500.0 "Noise")))
    (:`then_1`
      (if (`self.PlayCompletedSound`)
        (set `self.PlayCompletedSound` false)
        (`AudioComponent.Play` _completedsound 0.0)
        (`AISense_Hearing.ReportNoiseEvent` (`SceneComponent.K2_GetComponentLocation` _completedsound) 1.0 self 1500.0 "Noise")))
    (:`then_2`
      (if (`self.PlayButtonSound`)
        (set `self.PlayButtonSound` false)
        (`AudioComponent.Play` _buttonsound 0.0)
        (`AISense_Hearing.ReportNoiseEvent` (`SceneComponent.K2_GetComponentLocation` _buttonsound) 1.0 self 1500.0 "Noise")))))

(fn `UserConstructionScript`)