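; BP_ColoredCable is an electrical cable actor for the work-in-progress screw puzzle that makes impact sounds and AI-audible noise when it hits something.
; Tick caches the cable component's velocity each frame, and the hit event uses that previous-frame speed to ignore soft impacts.
; Hard hits play a random drop sound, unless one is already playing, with volume scaled by speed, and report a noise event at that location.
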(event `self.ReceiveTick`
  (params (DeltaSeconds :type "Float (single-precision)"))
  (set `self.LastFrameVelocity` (`SceneComponent.GetComponentVelocity` (`self.BP_ElectricalCableComp`))))

(event `self.BP_ElectricalCableComp.OnComponentHit`
  (params (HitComponent :type "PrimitiveComponent Object Reference") (OtherActor :type "Actor Object Reference") (OtherComp :type "PrimitiveComponent Object Reference") (NormalImpulse :type "Vector Structure") (Hit :type "HitResult Structure (by ref)"))
  (bind _groundhit (`self.GroundHit`))
  (bind _returnvalue (`KismetMathLibrary.VSize` (`self.LastFrameVelocity`)))
  (if (> _returnvalue 200.0)
    (if (not (`AudioComponent.IsPlaying` _groundhit))
      (bind _returnvalue_2 (`DroppableSoundComponent.SetRandomDropSound` (`self.DroppableSound`)))
      (`AudioComponent.SetSound` _groundhit _returnvalue_2)
      (`AudioComponent.SetVolumeMultiplier` _groundhit (/ _returnvalue 1000.0))
      (`AudioComponent.Play` _groundhit 0.0)
      (`AISense_Hearing.ReportNoiseEvent` (`SceneComponent.K2_GetComponentLocation` _groundhit) 1.0 self 0.0 "Noise"))))

(fn `UserConstructionScript`)