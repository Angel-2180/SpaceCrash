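; BP_ElectricalBox is an electrical box in the work-in-progress screw puzzle that gives audible feedback when cables connect to its four sockets.
; Tick polls each socket's PlayCableConnectedSound flag, clears it when set and plays the shared connection sound.
; It also reports a "Noise" event at the sound's location, which AI hearing can pick up.
; Despite its name, ActivateParticleEffects triggers no particles.
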(event `self.ReceiveBeginPlay`
  (`AudioComponent.Stop` (`self.CableConnectedSoundSocket`)))

(event `self.ReceiveTick`
  (params (DeltaSeconds :type "Float (single-precision)"))
  (`|ExecutionSequence`
    (:`then_0`
      (`self.ActivateParticleEffects` (`self.BP_ElectricalSocket`)))
    (:`then_1`
      (`self.ActivateParticleEffects` (`self.BP_ElectricalSocket1`)))
    (:`then_2`
      (`self.ActivateParticleEffects` (`self.BP_ElectricalSocket2`)))
    (:`then_3`
      (`self.ActivateParticleEffects` (`self.BP_ElectricalSocket3`)))))

(fn `ActivateParticleEffects`
  (params (SocketParent :type "/Game/Blueprints/ScrewPuzzle(WIP)/BP_ElectricalSocket Object Reference"))
  (bind _cableconnectedsoundsocket (`self.CableConnectedSoundSocket`))
  (if (`ElectricalSocketComponent.bPlayCableConnectedSound` SocketParent)
    (set `ElectricalSocketComponent.bPlayCableConnectedSound` false SocketParent)
    (`AudioComponent.Play` _cableconnectedsoundsocket 0.0)
    (`AISense_Hearing.ReportNoiseEvent` (`SceneComponent.K2_GetComponentLocation` _cableconnectedsoundsocket) 2.0 self 0.0 "Noise")))

(fn `UserConstructionScript`)