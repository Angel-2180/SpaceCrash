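; Cable link puzzle actor that gives audio and visual feedback for its four sockets.
; Each Tick it polls every socket's flags through a shared function, clearing each flag so effects fire once per trigger.
; The sound flag plays the cable-connected audio and reports a noise event at the audio component's location, which AI hearing can detect.
; The particle flag spawns sparks attached to that socket.
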(event `self.ReceiveBeginPlay`
  (`AudioComponent.Stop` (`self.CableConnectedSoundSocket`)))

(event `self.ReceiveTick`
  (params (DeltaSeconds :type "Float (single-precision)"))
  (`|ExecutionSequence`
    (:`then_0`
      (`self.ActivateParticleEffects` (`self.Socket 1`)))
    (:`then_1`
      (`self.ActivateParticleEffects` (`self.Socket 2`)))
    (:`then_2`
      (`self.ActivateParticleEffects` (`self.Socket 3`)))
    (:`then_3`
      (`self.ActivateParticleEffects` (`self.Socket 4`)))))

(fn `ActivateParticleEffects`
  (params (SocketParent :type "/Game/Blueprints/BP_WireSocket Object Reference"))
  (bind _cableconnectedsoundsocket (`self.CableConnectedSoundSocket`))
  (`|ExecutionSequence`
    (:`then_0`
      (if (`WireSocket.PlayCableConnectedSound` SocketParent)
        (set `WireSocket.PlayCableConnectedSound` false SocketParent)
        (`AudioComponent.Play` _cableconnectedsoundsocket 0.0)
        (`AISense_Hearing.ReportNoiseEvent` (`SceneComponent.K2_GetComponentLocation` _cableconnectedsoundsocket) 2.0 self 0.0 "Noise")))
    (:`then_1`
      (if (`WireSocket.IsParticleActive` SocketParent)
        (`GameplayStatics.SpawnEmitterAttached` "/Game/AssetsToPush/P_Sparks.P_Sparks" SocketParent "None" (0.0 0.0 2.0))
        (set `WireSocket.IsParticleActive` false SocketParent)))))

(fn `UserConstructionScript`)